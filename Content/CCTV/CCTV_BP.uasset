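; CCTV Blueprint that switches the player's view between six security cameras.
; ChangeCam takes a camera number, prints it, and sets player controller 0's view target to the matching CCTV reference without specifying a blend.
; The event graph does no work of its own, holding only empty events and an unconnected view-target call.
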(event `self.ReceiveBeginPlay`)

(fn `ChangeCam`
  (params (CCTVNum :type Integer))
  (`KismetSystemLibrary.PrintString` (`KismetStringLibrary.Conv_IntToString` CCTVNum))
  (switch `int` CCTVNum
    (:`1`
      (`PlayerController.SetViewTargetWithBlend` (`GameplayStatics.GetPlayerController` 0) (`self.CCTV1`) 0.0 "VTBlend_Linear" 0.0 false))
    (:`2`
      (`PlayerController.SetViewTargetWithBlend` (`GameplayStatics.GetPlayerController` 0) (`self.CCTV2`) 0.0 "VTBlend_Linear" 0.0 false))
    (:`3`
      (`PlayerController.SetViewTargetWithBlend` (`GameplayStatics.GetPlayerController` 0) (`self.CCTV3`) 0.0 "VTBlend_Linear" 0.0 false))
    (:`4`
      (`PlayerController.SetViewTargetWithBlend` (`GameplayStatics.GetPlayerController` 0) (`self.CCTV4`) 0.0 "VTBlend_Linear" 0.0 false))
    (:`5`
      (`PlayerController.SetViewTargetWithBlend` (`GameplayStatics.GetPlayerController` 0) (`self.CCTV5`) 0.0 "VTBlend_Linear" 0.0 false))
    (:`6`
      (`PlayerController.SetViewTargetWithBlend` (`GameplayStatics.GetPlayerController` 0) (`self.CCTV6`) 0.0 "VTBlend_Linear" 0.0 false))))

(fn `UserConstructionScript`)